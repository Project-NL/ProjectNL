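; Smoke volume actor that fills space with Niagara smoke sprites placed on voxel positions from a flood fill.
; Each tick it reruns FloodFill and pushes VoxelPositions into the SmokeVolume system's VectorArray.
; Sprite scale is derived from voxel size (target diameter over grid resolution).
; The construction script can optionally run the fill and show particles as an editor preview; its voxel debug drawing is disconnected.
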(event EventBeginPlay
  (Effects|Components|ParticleSystem|SetFloatParameter (Variables|Default|GetSmokeVolume) "SpriteUniformScale" (* (/ (Variables|Default|GetTargetVolumeDiameter) (Variables|Default|GetGridResolution)) 3.0)))

(event Collision|EventActorBeginOverlap
  (params (OtherActor :type Actor%20Object%20Reference)))

(event EventTick
  (params (DeltaSeconds :type Float%20%28single-precision%29))
  (Class|SmokeVolume|FloodFill)
  (Class|NiagaraDataInterfaceArrayFunctionLibrary|SetNiagaraArrayVector (Variables|Default|GetSmokeVolume) "VectorArray" (Variables|Default|GetVoxelPositions)))

(fn ConstructionScript
  (bind _smokevolume (Variables|Default|GetSmokeVolume))
  (if (Variables|Default|GetFloodFillOnConstruct)
    (Class|SmokeVolume|FloodFill)
    (Rendering|SetVisibility (Variables|Default|GetSmokeVolume) (Variables|Default|GetShowParticles) false)
    (if (Variables|Default|GetShowParticles)
      (Class|NiagaraDataInterfaceArrayFunctionLibrary|SetNiagaraArrayVector _smokevolume "VectorArray" (Variables|Default|GetVoxelPositions))
      (Effects|Components|ParticleSystem|SetFloatParameter _smokevolume "SpriteUniformScale" (* (/ (Variables|Default|GetTargetVolumeDiameter) (Variables|Default|GetGridResolution)) 3.0)))))